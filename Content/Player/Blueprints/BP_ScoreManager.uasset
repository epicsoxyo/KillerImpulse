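; BP_ScoreManager tracks the player's elapsed time as minutes and seconds and shows it as the score on the HUD.
; On BeginPlay it resets both counters in GI_KillerImPulseInstance, then starts the PlayEverySecond timeline.
; Each timeline trigger increments the seconds, rolls 60 over into a minute, and writes the formatted time to ScoreText through BP_Player's HUD reference.
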(event Custom|IncrementTimer
  (bind _gameinstance (Variables|Default|GetGameInstance))
  (bind _minutes (Variables|/Game/Levels/Blueprints/GI_KillerImPulseInstance.GI_KillerImPulseInstance_C|GetMinutes _gameinstance))
  (bind _result (Math|Integer|IncrementInt (Variables|/Game/Levels/Blueprints/GI_KillerImPulseInstance.GI_KillerImPulseInstance_C|GetSeconds _gameinstance))
    (:%20%20
      (if (== _result 60)
        (Variables|/Game/Levels/Blueprints/GI_KillerImPulseInstance.GI_KillerImPulseInstance_C|SetSeconds _gameinstance 0)
        (Math|Integer|IncrementInt _minutes
          (:%20%20
            _)))
      (bind _asbp_player (Utilities|Casting|CastToBP_Player (Game|GetPlayerCharacter 0)))
      (Rendering|Components|TextRender|SetText (Variables|/Game/UI/GameUI/KillerImpulseHUD.KillerImpulseHUD_C|GetScoreText (Variables|/Game/Player/Blueprints/BP_Player.BP_Player_C|GetHUDReference _asbp_player)) (Utilities|Text|FormatText "{Minutes}:{Seconds}" (Utilities|Text|ToText(Integer) _minutes false true 2 2) (Utilities|Text|ToText(Integer) (Variables|/Game/Levels/Blueprints/GI_KillerImPulseInstance.GI_KillerImPulseInstance_C|GetSeconds _gameinstance) false true 2 2))))))

(event EventBeginPlay
  (Variables|Default|SetCustomTimeDilation 1.0)
  (bind _asgi_killer_im_pulse_instance (Utilities|Casting|CastToGI_KillerImPulseInstance (Game|GetGameInstance)))
  (bind _output_get (Variables|Default|SetGameInstance _asgi_killer_im_pulse_instance))
  (Variables|/Game/Levels/Blueprints/GI_KillerImPulseInstance.GI_KillerImPulseInstance_C|SetSeconds _output_get 0)
  (Variables|/Game/Levels/Blueprints/GI_KillerImPulseInstance.GI_KillerImPulseInstance_C|SetMinutes _output_get 0)
  (Timeline|PlayEverySecond Play
    (:Trigger%20Event
      (CallFunction|IncrementTimer))))

(fn ConstructionScript)
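; Player character that moves and looks via Enhanced Input and can stop alarms on nearby alarm boxes.
; BeginPlay adds the input mapping, creates the KillerImpulseHUD twice (heart rate and score functions, only the latter stored), then opens HypeRateMenu with the game paused.
; Capsule overlaps track the last entered BP_AlarmBox as the interact target, without comparing distances.
; Pause creates the menu if needed, switches to UI-only input and pauses the game.
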(event OnComponentBeginOverlap(CapsuleComponent)
  (params (OverlappedComponent :type Primitive%20Component%20Object%20Reference) (OtherActor :type Actor%20Object%20Reference) (OtherComp :type Primitive%20Component%20Object%20Reference) (OtherBodyIndex :type Integer) (bFromSweep :type Boolean) (SweepResult :type Hit%20Result%20Structure%20%28by%20ref%29))
  (bind _asbp_alarm_box (Utilities|Casting|CastToBP_AlarmBox OtherActor))
  (Utilities|IsValid _asbp_alarm_box
    (:Is%20Valid
      (Variables|Default|SetClosestAlarmBox _asbp_alarm_box))))

(event OnComponentEndOverlap(CapsuleComponent)
  (params (OverlappedComponent :type Primitive%20Component%20Object%20Reference) (OtherActor :type Actor%20Object%20Reference) (OtherComp :type Primitive%20Component%20Object%20Reference) (OtherBodyIndex :type Integer))
  (bind _asbp_alarm_box (Utilities|Casting|CastToBP_AlarmBox OtherActor))
  (Utilities|IsValid _asbp_alarm_box
    (:Is%20Valid
      (if (== _asbp_alarm_box (Variables|Default|GetClosestAlarmBox))
        (Variables|Default|SetClosestAlarmBox 0)))))

(event Input|EnhancedActionEvents|EnhancedInputActionIA_Pause
  (params (ActionValue :type Boolean) (ElapsedSeconds :type Float%20%28double-precision%29) (TriggeredSeconds :type Float%20%28double-precision%29) (InputAction :type Input%20Action%20Object%20Reference :default "/Game/Player/Input/Actions/IA_Pause.IA_Pause"))
  (:Triggered
    (Utilities|IsValid (Variables|Default|GetMenuReference)
      (:Is%20Valid
        _)
      (:Is%20Not%20Valid
        (|CreateMenu)))
    (|FocusOnMenu)))

(event Input|EnhancedActionEvents|EnhancedInputActionIA_Interact
  (params (ActionValue :type Boolean) (ElapsedSeconds :type Float%20%28double-precision%29) (TriggeredSeconds :type Float%20%28double-precision%29) (InputAction :type Input%20Action%20Object%20Reference :default "/Game/Player/Input/Actions/IA_Interact.IA_Interact"))
  (bind _closestalarmbox (Variables|Default|GetClosestAlarmBox))
  (:Triggered
    (Utilities|IsValid _closestalarmbox
      (:Is%20Valid
        (Default|StopAlarm _closestalarmbox)))))

(event Input|EnhancedActionEvents|EnhancedInputActionIA_Look
  (params (ActionValue :type Vector%202D%20Structure) (ElapsedSeconds :type Float%20%28double-precision%29) (TriggeredSeconds :type Float%20%28double-precision%29) (InputAction :type Input%20Action%20Object%20Reference :default "/Game/Player/Input/Actions/IA_Look.IA_Look"))
  (:Triggered
    (Pawn|Input|AddControllerYawInput (.x ActionValue))
    (Pawn|Input|AddControllerPitchInput (.y ActionValue))))

(event Input|EnhancedActionEvents|EnhancedInputActionIA_Move
  (params (ActionValue :type Vector%202D%20Structure) (ElapsedSeconds :type Float%20%28double-precision%29) (TriggeredSeconds :type Float%20%28double-precision%29) (InputAction :type Input%20Action%20Object%20Reference :default "/Game/Player/Input/Actions/IA_Move.IA_Move"))
  (:Triggered
    (|MoveRight (.x ActionValue))
    (|MoveForward (.y ActionValue))))

(event EventBeginPlay
  (|AddMappingContextToEIC)
  (|HeartRateWidget)
  (|ScoreWidget)
  (|MainMenu))

(fn ConstructionScript)
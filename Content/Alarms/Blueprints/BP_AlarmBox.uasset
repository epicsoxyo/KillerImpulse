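; Alarm box actor that shows a ringing alarm clock with a 15-second countdown, ending in player death if not stopped.
; AddAlarm starts the sound and KillAfterSeconds timeline, updates the clock face, and adds a fade-out widget when time expires.
; A radius overlap shows prompt text while the player is near an active alarm.
; StopAlarm silences and hides it, then calls CallSpawnAlarm after a short delay.
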(event OnComponentBeginOverlap(StoppingRadius)
  (params (OverlappedComponent :type Primitive%20Component%20Object%20Reference) (OtherActor :type Actor%20Object%20Reference) (OtherComp :type Primitive%20Component%20Object%20Reference) (OtherBodyIndex :type Integer) (bFromSweep :type Boolean) (SweepResult :type Hit%20Result%20Structure%20%28by%20ref%29))
  (bind _asbp_player (Utilities|Casting|CastToBP_Player OtherActor))
  (Utilities|IsValid _asbp_player
    (:Is%20Valid
      (Variables|Default|SetplayerIsNearby true)
      (if (Variables|Default|GethasAlarm)
        (Rendering|SetVisibility (Variables|Default|GetTextRender) true true)))))

(event OnComponentEndOverlap(StoppingRadius)
  (params (OverlappedComponent :type Primitive%20Component%20Object%20Reference) (OtherActor :type Actor%20Object%20Reference) (OtherComp :type Primitive%20Component%20Object%20Reference) (OtherBodyIndex :type Integer))
  (bind _asbp_player (Utilities|Casting|CastToBP_Player OtherActor))
  (Utilities|IsValid _asbp_player
    (:Is%20Valid
      (Variables|Default|SetplayerIsNearby false)
      (Rendering|SetVisibility (Variables|Default|GetTextRender) false true))))

(event Custom|AddAlarm
  (Variables|Default|SethasAlarm true)
  (Rendering|SetVisibility (Variables|Default|GetSM_AlarmClock) true true)
  (Audio|Components|Audio|Play (Variables|Default|GetA_AlarmClock) 0.0)
  (if (Variables|Default|GetplayerIsNearby)
    (Rendering|SetVisibility (Variables|Default|GetTextRender) true true))
  (Variables|Default|SetcountdownValue 15)
  (Timeline|KillAfterSeconds PlayFromStart
    (:Finished
      (CallFunction|KillPlayer))
    (:_
      (|DecrementClockFace))))

(event Custom|KillPlayer
  (bind _returnvalue (UserInterface|CreateWidget "/Game/Levels/Blueprints/BP_FadeOut.BP_FadeOut_C"))
  (UserInterface|Viewport|AddtoViewport _returnvalue 1))

(event Custom|StopAlarm
  (Audio|PlaySoundatLocation "/Game/Alarms/Audio/SW_ButtonClick.SW_ButtonClick" (Transformation|GetWorldLocation (Variables|Default|GetSM_AlarmClock)) "0, 0, 0" 1.0 1.0 0.0 "/Game/Alarms/Audio/SA_AlarmClock.SA_AlarmClock" 0 0 0)
  (Variables|Default|SethasAlarm false)
  (Rendering|SetVisibility (Variables|Default|GetTextRender) false true)
  (Rendering|SetVisibility (Variables|Default|GetSM_AlarmClock) false true)
  (Audio|Components|Audio|Stop (Variables|Default|GetA_AlarmClock))
  (Audio|Components|Audio|Stop (Variables|Default|GetKillAfterSeconds))
  (Utilities|FlowControl|Delay 3.0)
  (Default|CallSpawnAlarm))

(fn ConstructionScript
  (Variables|Default|SetCustomTimeDilation 1.0)
  (Rendering|SetVisibility (Variables|Default|GetSM_AlarmClock) false true)
  (Rendering|SetVisibility (Variables|Default|GetTextRender) false true))
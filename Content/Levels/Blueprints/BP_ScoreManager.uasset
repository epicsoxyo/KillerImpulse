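; Score manager actor that tracks elapsed time as the score, stored as minutes and seconds in GI_KillerImPulseInstance.
; BeginPlay resets both counters, then the PlayEverySecond timeline's event increments seconds and rolls them into minutes.
; Each tick of that event sets BP_Player's HUD score text from GetScoreString, whose minutes:seconds format node appears unconnected.
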(event EventBeginPlay
  (Variables|Default|SetCustomTimeDilation 1.0)
  (bind _gameinstance (|SetGameInstance))
  (|ResetScore _gameinstance)
  (Timeline|PlayEverySecond Play
    (:Trigger%20Event
      (|IncrementScore))))

(fn ConstructionScript)
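; Enemy AI controller that switches between chasing the player and patrolling random navigable points.
; A looping one-second timer picks Patrol or ChasePlayer using IsChasing and two distance checks, though nothing here sets that flag.
; Both distance functions compare pawn-to-player distance against their thresholds, but those comparisons are left unused.
; Patrol picks points around the world origin and, unlike ChasePlayer, passes no pawn to AIMoveTo.
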(event Custom|TrackPlayer
  (if (Variables|Default|GetIsChasing)
    (if (|IsInPatrollingDistance)
      (|Patrol :!label _label)
      (else
        (|ChasePlayer :!label _label_2)))
    (elif (|IsInChasingDistance)
      (goto _label_2)
      (else
        (goto _label)))))

(event EventBeginPlay
  (Utilities|Time|SetTimerbyEvent (delegate Custom|TrackPlayer) 1.0 true))

(fn ConstructionScript)
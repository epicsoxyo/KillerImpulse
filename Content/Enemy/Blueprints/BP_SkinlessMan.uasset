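; BP_SkinlessMan is an enemy that attacks the player at close range and presents the player's death.
; Player overlaps with its HitRadius start the attack animation in ABP_SkinlessMan, and leaving calls that blueprint's end-of-animation handler.
; On BeginPlay it binds to the anim blueprint's player-died event, which plays a punch sound and adds a fade-out widget to the screen.
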(event OnComponentBeginOverlap(HitRadius)
  (params (OverlappedComponent :type Primitive%20Component%20Object%20Reference) (OtherActor :type Actor%20Object%20Reference) (OtherComp :type Primitive%20Component%20Object%20Reference) (OtherBodyIndex :type Integer) (bFromSweep :type Boolean) (SweepResult :type Hit%20Result%20Structure%20%28by%20ref%29))
  (bind _asbp_player (Utilities|Casting|CastToBP_Player OtherActor))
  (Utilities|IsValid _asbp_player
    (:Is%20Valid
      (bind _asabp_skinless_man (Utilities|Casting|CastToABP_SkinlessMan (Components|SkeletalMesh|GetAnimInstance (Variables|Character|GetMesh))))
      (Utilities|IsValid _asabp_skinless_man
        (:Is%20Valid
          (Default|AttackAnimation _asabp_skinless_man))))))

(event OnComponentEndOverlap(HitRadius)
  (params (OverlappedComponent :type Primitive%20Component%20Object%20Reference) (OtherActor :type Actor%20Object%20Reference) (OtherComp :type Primitive%20Component%20Object%20Reference) (OtherBodyIndex :type Integer))
  (bind _asbp_player (Utilities|Casting|CastToBP_Player OtherActor))
  (Utilities|IsValid _asbp_player
    (:Is%20Valid
      (bind _asabp_skinless_man (Utilities|Casting|CastToABP_SkinlessMan (Components|SkeletalMesh|GetAnimInstance (Variables|Character|GetMesh))))
      (Utilities|IsValid _asabp_skinless_man
        (:Is%20Valid
          (Default|AnimNotifyEndOfAnim _asabp_skinless_man))))))

(event Custom|Die
  (Audio|PlaySound2D "/Game/Enemy/Audio/SW_Punch.SW_Punch" 1.0 1.0 0.0 0 0)
  (bind _returnvalue (UserInterface|CreateWidget "/Game/Levels/Blueprints/BP_FadeOut.BP_FadeOut_C"))
  (UserInterface|Viewport|AddtoViewport _returnvalue 1))

(event EventBeginPlay
  (bind _asabp_skinless_man (Utilities|Casting|CastToABP_SkinlessMan (Components|SkeletalMesh|GetAnimInstance (Variables|Character|GetMesh))))
  (EventDispatchers|BindEventtoPlayerDied _asabp_skinless_man (delegate Custom|Die)))

(fn ConstructionScript)